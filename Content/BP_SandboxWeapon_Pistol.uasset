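; Sandbox pistol weapon Blueprint that handles single-shot hitscan firing.
; SandboxFire checks CanFire and ammo, then plays a sound, line-traces along the FirePoint forward vector and updates ammo.
; A timer derived from RoF calls HandleFireDelay to pace shots, with CanFire cleared meanwhile.
; An empty magazine triggers a reload with sound; BeginPlay also calls Fire once after a short delay.
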(event EventSandboxFire
  (if (Variables|Default|GetCanFire)
    (bind _returnvalue (Class|SandboxWeaponBase|CheckAmmo))
    (if _returnvalue
      (Utilities|FlowControl|Sequence
        (:then_0
          (Class|SandboxWeaponBase|PlaySound)
          (Class|SandboxWeaponBase|LinetraceOneShot (Math|Vector|GetForwardVector (Variables|Default|GetFirePoint)))
          (Class|SandboxWeaponBase|UpdateAmmo))
        (:then_1
          (bind _returnvalue_2 (Utilities|Time|SetTimerbyFunctionName 0 "HandleFireDelay" (/ 1.0 (Variables|Default|GetRoF))))
          (Variables|Default|SetTimerFireDelay _returnvalue_2)
          (Variables|Default|SetCanFire false)))
      (else
        (Class|SandboxWeaponBase|Reload)
        ;[0.15 0.15 0.15 0.5] 장전 사운드
        (Class|SandboxWeaponBase|PlaySound)))))

(event EventBeginPlay
  (Utilities|FlowControl|Delay 2.0)
  (Class|WeaponBase|Fire))

(fn ConstructionScript)
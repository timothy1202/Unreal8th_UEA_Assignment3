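; Shotgun template weapon Blueprint that overrides its parent's firing, reload and effects events.
; ProcessFiring casts six debug-drawn Visibility line traces randomly spread in a forward cone, ignoring the owner and applying damage to each hit actor.
; PlayEffects plays a sound at the actor's location, while Reload only calls the parent.
; BeginPlay holds test code that fires after a delay and prints a message, leaving the parent BeginPlay call disconnected.
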(event EventReload
  ;[0.15 0.15 0.15 0.5] 블루프린트 부모만 작동
  (|CallParentFunction))

(event EventPlayEffects
  (Audio|PlaySoundatLocation "/Engine/EditorSounds/GamePreview/EjectFromPlayer_Cue.EjectFromPlayer_Cue" (Transformation|GetActorLocation) "0, 0, 0" 1.0 1.0 0.0 0 0 0 0))

(event EventProcessFiring
  (bind _root (Variables|Default|GetRoot))
  (bind _returnvalue (Transformation|GetWorldLocation _root))
  (for _index (range 1 6)
    (bind (_outhit _returnvalue_2) (Collision|LineTraceByChannel _returnvalue (+ _returnvalue (* (Math|Random|RandomUnitVectorinConeinDegrees (Math|Vector|GetForwardVector _root) 2e+01) (Variables|Default|GetRange))) "TraceTypeQuery1" false (Utilities|Array|MakeArray (Components|GetOwner)) "ForDuration"))
    (if _returnvalue_2
      (Game|Damage|ApplyDamage (.HitActor (Collision|BreakHitResult _outhit)) (Variables|Default|GetDamagePerHit) 0 0))))

(event EventBeginPlay
  (Utilities|FlowControl|Delay 5.0)
  (Class|WeaponBase|Fire)
  (Development|PrintString "Hello"))

(fn ConstructionScript)